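; Mana potion pickup actor that applies an instant Gameplay Effect to whatever actor overlaps its sphere and respawns in place.
; The sphere overlap passes the other actor to ApplyEffectToTarget with the configured effect class, with no filtering in this graph.
; It then turns off sphere overlaps and hides the mesh, restoring both after a short delay instead of destroying the actor.
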(event `self.Sphere.OnComponentBeginOverlap`
  (params (OverlappedComponent :type "PrimitiveComponent Object Reference") (OtherActor :type "Actor Object Reference") (OtherComp :type "PrimitiveComponent Object Reference") (OtherBodyIndex :type Integer) (bFromSweep :type Boolean) (SweepResult :type "HitResult Structure (by ref)"))
  (`self.ApplyEffectToTarget` OtherActor (`self.InstantGameplayEffectClass`))
  (set `PrimitiveComponent.bGenerateOverlapEvents` false (`self.Sphere`))
  (`SceneComponent.SetVisibility` (`self.PotionMesh`) false false)
  (`KismetSystemLibrary.Delay` 3.0)
  (`SceneComponent.SetVisibility` (`self.PotionMesh`) true false)
  (set `PrimitiveComponent.bGenerateOverlapEvents` true (`self.Sphere`)))

(fn `UserConstructionScript`)