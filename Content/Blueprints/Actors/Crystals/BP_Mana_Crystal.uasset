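; Mana crystal pickup actor that applies a duration Gameplay Effect to any actor overlapping its box collider, with no filtering on the overlapping actor.
; On overlap it calls ApplyEffectToTarget with the duration effect class, then turns off overlap events and hides the mesh.
; After a three-second delay it restores both, so the same actor acts as a respawning pickup without being destroyed.
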(event `self.BoxCollider.OnComponentBeginOverlap`
  (params (OverlappedComponent :type "PrimitiveComponent Object Reference") (OtherActor :type "Actor Object Reference") (OtherComp :type "PrimitiveComponent Object Reference") (OtherBodyIndex :type Integer) (bFromSweep :type Boolean) (SweepResult :type "HitResult Structure (by ref)"))
  (`self.ApplyEffectToTarget` OtherActor (`self.DurationGameplayEffectClass`))
  (set `PrimitiveComponent.bGenerateOverlapEvents` false (`self.BoxCollider`))
  (`SceneComponent.SetVisibility` (`self.CrystalMesh`) false false)
  (`KismetSystemLibrary.Delay` 3.0)
  (`SceneComponent.SetVisibility` (`self.CrystalMesh`) true false)
  (set `PrimitiveComponent.bGenerateOverlapEvents` true (`self.BoxCollider`)))

(fn `UserConstructionScript`)